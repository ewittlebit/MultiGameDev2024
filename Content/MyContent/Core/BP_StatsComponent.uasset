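; BP_StatsComponent is a stats component that holds an owner's Health and MaxHealth.
; SetHealth clamps between zero and MaxHealth, while SetMaxHealth floors the maximum at zero without re-clamping Health.
; Both setters and the RepNotify functions for both values fire OnHealthChanged, so replicated changes also reach listeners.
; GetHealth returns both values, and the component does no work on BeginPlay or Tick.
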(event EventBeginPlay)

(event EventTick
  (params (DeltaSeconds :type Float%20%28single-precision%29)))

(fn SetHealth
  (params (Health :type Integer))
  (Variables|Default|SetHealth (Math|Integer|Clamp(Integer) Health 0 (Variables|Default|GetMaxHealth)))
  (Default|CallOnHealthChanged))

(fn SetMaxHealth
  (params (MaxHealth :type Integer))
  (Variables|Default|SetMaxHealth (Math|Integer|Max(Integer) MaxHealth))
  (Default|CallOnHealthChanged))

(fn GetHealth
  (return (Variables|Default|GetHealth) (Variables|Default|GetMaxHealth)))

(fn OnRepHealth
  (Default|CallOnHealthChanged))

(fn OnRepMaxHealth
  (Default|CallOnHealthChanged))