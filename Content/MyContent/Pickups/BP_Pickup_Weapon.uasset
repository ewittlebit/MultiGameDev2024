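; BP_Pickup_Weapon is a pickup that gives a weapon to the character that activates it.
; When OnActivatePickup fires, it casts the pickup actor to BP_Character and calls ActivateWeapon with its WeaponClass.
; Any other actor type is ignored, and the BeginPlay, overlap and Tick events are disabled stubs with no logic of their own.
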(event EventBeginPlay
  (|CallParentFunction) ; This node is disabled and will not be called.\nDrag off pins to build functionality.
)

(event Collision|EventActorBeginOverlap
  (params (OtherActor :type Actor%20Object%20Reference))
  (|CallParentFunction OtherActor) ; This node is disabled and will not be called.\nDrag off pins to build functionality.
)

(event EventTick
  (params (DeltaSeconds :type Float%20%28single-precision%29))
  (|CallParentFunction DeltaSeconds) ; This node is disabled and will not be called.\nDrag off pins to build functionality.
)

(event EventOnActivatePickup
  (params (pickupActor :type Actor%20Object%20Reference))
  (bind _asbp_character (Utilities|Casting|CastToBP_Character pickupActor))
  (Default|ActivateWeapon _asbp_character (Variables|Default|GetWeapon%20Class)))

(fn ConstructionScript
  (|CallParentFunction))