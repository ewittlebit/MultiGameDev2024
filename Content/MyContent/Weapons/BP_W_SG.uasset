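; BP_W_SG is a weapon Blueprint, likely a shotgun, that fires several hitscan shots per trigger event.
; Its FiredOnServer function calls ApplyLineTraceDamage once for each of BulletsPerShot, then starts a single cooldown when that count is above zero.
; The trace, damage and cooldown helpers are not defined here, and the event graph and construction script add no logic of their own.
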(event EventBeginPlay
  (|CallParentFunction) ; This node is disabled and will not be called.\nDrag off pins to build functionality.
)

(event Collision|EventActorBeginOverlap
  (params (OtherActor :type Actor%20Object%20Reference))
  (|CallParentFunction OtherActor) ; This node is disabled and will not be called.\nDrag off pins to build functionality.
)

(event EventTick
  (params (DeltaSeconds :type Float%20%28single-precision%29))
  (|CallParentFunction DeltaSeconds) ; This node is disabled and will not be called.\nDrag off pins to build functionality.
)

(fn ConstructionScript
  (|CallParentFunction))

(fn FiredonServer
  (if (> (Variables|Default|GetBulletsPerShot) 0)
    (for _index (range 0 (- (Variables|Default|GetBulletsPerShot) 1))
      (CallFunction|ApplyLineTraceDamage "None"))
    (CallFunction|StartCooldown)))