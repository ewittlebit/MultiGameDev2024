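; Player State Blueprint that holds a player's kill count and display name.
; Both values use RepNotify functions that fire OnKillsUpdated and OnPlayerDisplayNameUpdated, so listeners can react to replicated changes.
; The setters also fire these notifications directly after writing the value, and AddKill increments the count through SetKills.
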(fn ConstructionScript)

(fn OnRepKills
  (Default|CallOnKillsUpdated))

(fn OnRepPlayerDisplayName
  (Default|CallOnPlayerDisplayNameUpdated))

(fn SetKills
  (params (Kills :type Integer))
  (Variables|Default|SetKills Kills)
  (Default|CallOnKillsUpdated))

(fn SetPlayerDisplayName
  (params (PlayerDisplayName :type String))
  (Variables|Default|SetPlayerDisplayName PlayerDisplayName)
  (Default|CallOnPlayerDisplayNameUpdated))

(fn AddKill
  (CallFunction|SetKills (+ (Variables|Default|GetKills) 1)))